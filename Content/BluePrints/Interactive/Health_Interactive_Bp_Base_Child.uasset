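; A child of the interactive health base Blueprint, a pickup that restores a fixed amount of health to the player on interaction.
; Interact adds health to the player and refreshes the health widget.
; It then plays its audio, disables actor collision and jumps the animation instance to a Destroy node.
; BeginPlay stops the audio so it stays silent until use.
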(event EventBeginPlay
  (Audio|Components|Audio|Stop (Variables|Default|GetAudio)))

(event Collision|EventActorBeginOverlap
  (params (OtherActor :type Actor%20Object%20Reference)))

(event EventTick
  (params (DeltaSeconds :type Float%20%28single-precision%29)))

(fn ConstructionScript
  (|CallParentFunction))

(fn Interact
  (params (Player%20Ref :type BP%20Player%20Object%20Reference))
  (Default|AddHealth Player%20Ref 25.0)
  (Default|HealthWidgetUpdate Player%20Ref)
  (Audio|Components|Audio|Play (Variables|Default|GetAudio) 0.0)
  (Collision|SetActorEnableCollision false)
  (Class|PaperZDAnimInstance|JumptoNode (Variables|/Script/PaperZD.PaperZDAnimationComponent|GetAnimInstance (Variables|Default|GetAnimationComponent)) "Destroy" "None"))