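; Base enemy Blueprint that tracks health and death and provides distance-based footstep audio.
; Construction fills health from its default; damage lowers it within bounds and fires the currently empty EnemyDied once at zero.
; UpdateFootstepVolume, not called here, scales volume directly with player distance, louder when farther, and mutes it with a debug print beyond range.
; The capsule overlap handler is empty.
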(event OnComponentBeginOverlap(CapsuleComponent)
  (params (OverlappedComponent :type Primitive%20Component%20Object%20Reference) (OtherActor :type Actor%20Object%20Reference) (OtherComp :type Primitive%20Component%20Object%20Reference) (OtherBodyIndex :type Integer) (bFromSweep :type Boolean) (SweepResult :type Hit%20Result%20Structure%20%28by%20ref%29)))

(event Game|Damage|EventAnyDamage
  (params (Damage :type Float%20%28single-precision%29) (DamageType :type Damage%20Type%20Object%20Reference) (InstigatedBy :type Controller%20Object%20Reference) (DamageCauser :type Actor%20Object%20Reference))
  (Variables|Default|SetHealth (Math|Float|Clamp(Float) (- (Variables|Default|GetHealth) Damage) 0.0 (Variables|Default|GetDefualtHealth)))
  (if (and (<= (Variables|Default|GetHealth) 0.0) (not (Variables|Default|GetisDead)))
    (Variables|Default|SetisDead true)
    (CallFunction|EnemyDied)))

(fn ConstructionScript
  (Variables|Default|SetHealth (Variables|Default|GetDefualtHealth))
  (Variables|Default|SetSelf_0 self))

(fn EnemyDied)

(fn UpdateFootstepVolume
  (bind _returnvalue (Game|GetPlayerCharacter 0))
  (bind _self_0 (Variables|Default|GetSelf_0))
  (bind _footstepsound (Variables|Default|GetFootstepSound))
  (bind _returnvalue_2 (Transformation|GetDistanceTo _returnvalue _self_0))
  (if (<= _returnvalue_2 8e+02)
    (Audio|Components|Audio|AdjustVolume _footstepsound 0.0 (Math|Float|NormalizetoRange (/ _returnvalue_2 8e+02) 0.0 1.0) "Linear" :!class /Script/Engine.AudioComponent)
    (else
      (Development|PrintString "Hello")
      (Audio|Components|Audio|AdjustVolume _footstepsound 0.0 0.0 "Linear" :!class /Script/Engine.AudioComponent))))