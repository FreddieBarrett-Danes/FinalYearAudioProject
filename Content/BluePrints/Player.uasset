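; Player character Blueprint that handles movement, jumping and flipbook sprite animation.
; MoveForward and MoveRight axes add movement along fixed world axes, while the Jumping action starts and stops jumps.
; Tick and jump input pick the jump, run or idle flipbook from falling state and velocity.
; Tick also flips the controller yaw by the sign of Y velocity, so the sprite faces its lateral travel direction.
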(event Custom|UpdateAnimation
  (Sprite|SetFlipbook (Variables|Default|GetSprite) (select (AI|Components|NavMovement|IsFalling (Variables|Character|GetCharacterMovement)) "/Game/ImportedContent/SunnyLandAssets/sprites/player/jump/player-jump.player-jump" (select (> (Math|Vector|VectorLength (Variables|/Script/Engine.MovementComponent|GetVelocity (Variables|Character|GetCharacterMovement))) 0.0) "/Game/ImportedContent/SunnyLandAssets/sprites/player/run/player-run.player-run" "/Game/ImportedContent/SunnyLandAssets/sprites/player/idle/player-idle.player-idle"))))

(event Custom|UpdateRotation
  (Utilities|IsValid (Pawn|GetController)
    (:Is%20Valid
      (Math|Float|CompareFloat (.Y (Class|KismetMathLibrary|BreakVector3f (Variables|/Script/Engine.MovementComponent|GetVelocity (Variables|Character|GetCharacterMovement)))) 0.0
        (:>
          (Pawn|SetControlRotation (Pawn|GetController) (Math|Rotator|MakeRotator 0.0 0.0 0.0)))
        (:<
          (Pawn|SetControlRotation (Pawn|GetController) (Math|Rotator|MakeRotator 0.0 0.0 1.8e+02)))))))

(event EventBeginPlay)

(event Collision|EventActorBeginOverlap
  (params (OtherActor :type Actor%20Object%20Reference)))

(event EventTick
  (params (DeltaSeconds :type Float%20%28single-precision%29))
  (CallFunction|UpdateAnimation)
  (CallFunction|UpdateRotation))

(event Input|ActionEvents|InputActionJumping
  (params (Key :type Key%20Structure :default "None"))
  (:Pressed
    (Character|Jump)
    (Sprite|SetFlipbook (Variables|Default|GetSprite) (select (AI|Components|NavMovement|IsFalling (Variables|Character|GetCharacterMovement)) "/Game/ImportedContent/SunnyLandAssets/sprites/player/jump/player-jump.player-jump" (select (> (Math|Vector|VectorLength (Variables|/Script/Engine.MovementComponent|GetVelocity (Variables|Character|GetCharacterMovement))) 0.0) "/Game/ImportedContent/SunnyLandAssets/sprites/player/run/player-run.player-run" "/Game/ImportedContent/SunnyLandAssets/sprites/player/idle/player-idle.player-idle")) :!label _label))
  (:Released
    (Character|StopJumping)
    (goto _label)))

(event Input|AxisEvents|InputAxisMoveRight
  (params (AxisValue :type Float%20%28single-precision%29))
  (Pawn|Input|AddMovementInput "0.000000,-1.000000,0.000000" AxisValue false))

(event Input|AxisEvents|InputAxisMoveForward
  (params (AxisValue :type Float%20%28single-precision%29))
  (Pawn|Input|AddMovementInput "1.000000,0.000000,0.000000" AxisValue false))

(fn ConstructionScript)